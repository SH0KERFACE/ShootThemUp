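; BP_STUPlayerCharacter is the player character Blueprint that relays weapon firing from the controlling player to other machines.
; On BeginPlay it binds to the WeaponComponent's start and stop fire delegates, which call server events that in turn call multicast events, as their names indicate.
; The multicast events start or stop the current weapon only where the character is not locally controlled, so the firing player's own shot is not repeated.
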(event Custom|StartFire_Multi
  (if (not (Pawn|IsLocallyControlled))
    (Class|STUBaseWeapon|StartFire (Variables|/Script/ShootThemUp.STUWeaponComponent|GetCurrentWeapon (Variables|Default|GetWeaponComponent)))))

(event Custom|StopFire_Multi
  (if (not (Pawn|IsLocallyControlled))
    (Class|STUBaseWeapon|StopFire (Variables|/Script/ShootThemUp.STUWeaponComponent|GetCurrentWeapon (Variables|Default|GetWeaponComponent)))))

(event Custom|OnStopFire_Event
  (CallFunction|StopFireServ))

(event Custom|OnStartFire_Event
  (CallFunction|StartFireServ))

(event Custom|StartFire_Serv
  (CallFunction|StartFireMulti))

(event Custom|StopFire_Serv
  (CallFunction|StopFireMulti))

(event EventBeginPlay
  (bind _weaponcomponent (Variables|Default|GetWeaponComponent))
  (EventDispatchers|AssignOnStartFire _weaponcomponent (delegate Custom|OnStartFire_Event))
  (EventDispatchers|AssignOnStopFire _weaponcomponent (delegate Custom|OnStopFire_Event)))

(fn ConstructionScript)