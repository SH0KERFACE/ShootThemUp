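; Player controller Blueprint that handles respawning the player's character.
; BeginPlay caches the BP_STUGameState reference.
; RestartPlayer unpossesses the current pawn, gets a random game start from that game state, then spawns a new BP_STUPlayerCharacter at its location with always-spawn collision handling and possesses it.
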(event EventBeginPlay
  (|CallParentFunction)
  (bind _asbp_stugame_state (Utilities|Casting|CastToBP_STUGameState (Game|GetGameState)))
  (Variables|Default|SetAs%20BP%20STUGame%20State _asbp_stugame_state))

(fn ConstructionScript)

(fn RestartPlayer
  (bind _as_bp_stugame_state (Variables|Default|GetAs%20BP%20STUGame%20State))
  (Pawn|UnPossess)
  (Utilities|IsValid _as_bp_stugame_state
    (:Is%20Valid
      (bind _gamestart (Default|GetRandomGameStart _as_bp_stugame_state))
      (bind _returnvalue (Game|SpawnActorfromClass "/Game/Player/BP_STUPlayerCharacter.BP_STUPlayerCharacter_C" (Math|Transform|MakeTransform (Transformation|GetActorLocation _gamestart) "0, 0, 0" "1.000000,1.000000,1.000000") "AlwaysSpawn" "MultiplyWithRoot" 0 0))
      (Pawn|Possess _returnvalue))))