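; BP_Projectile is a weapon projectile that explodes on impact, dealing radial damage.
; When its sphere component hits, it stops movement, applies damage around its location credited to its owner's instigator controller, and spawns explosion FX at the impact point.
; It destroys itself after a short delay.
; InitVelocity_Multicast sets the movement component's velocity, with its name indicating a multicast to clients.
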(event OnComponentHit(Sphere)
  (params (HitComponent :type Primitive%20Component%20Object%20Reference) (OtherActor :type Actor%20Object%20Reference) (OtherComp :type Primitive%20Component%20Object%20Reference) (NormalImpulse :type Vector :default "0, 0, 0") (Hit :type Hit%20Result%20Structure%20%28by%20ref%29))
  (Components|Movement|StopMovementImmediately (Variables|Default|GetProjectileMovement))
  (Game|Damage|ApplyRadialDamage (Variables|Default|GetMaxDamage) (Transformation|GetActorLocation) (Variables|Default|GetDamageRadius) 0 0 self (Game|GetInstigatorController (Components|GetOwner)) (Variables|Default|GetDo%20Full%20Damage) "ECC_Visibility")
  (Niagara|SpawnSystematLocation (Variables|Default|GetExplodeFX) (.ImpactPoint (Collision|BreakHitResult Hit)))
  (Utilities|FlowControl|Delay 0.1)
  (Actor|DestroyActor))

(event Custom|InitVelocity_Multicast
  (params (Velocity :type Vector))
  (Variables|/Script/Engine.MovementComponent|SetVelocity (Variables|Default|GetProjectileMovement) Velocity))

(event EventBeginPlay)

(event Collision|EventActorBeginOverlap
  (params (OtherActor :type Actor%20Object%20Reference)))

(fn ConstructionScript)