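; Launcher weapon Blueprint that fires one projectile per StartFire, with StopFire left empty.
; Fire plays a no-ammo sound when empty, otherwise spawns muzzle FX and decrements ammo.
; Only the server spawns the projectile at the muzzle, then sets its velocity through a multicast call.
; Direction runs from the muzzle to the aim trace's impact point, or to the trace end without a blocking hit.
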(event EventBeginPlay)

(event Collision|EventActorBeginOverlap
  (params (OtherActor :type Actor%20Object%20Reference)))

(event EventTick
  (params (DeltaSeconds :type Float%20%28single-precision%29)))

(event EventStartFire
  (params (Character :type STU%20Base%20Character%20Object%20Reference))
  (CallFunction|Fire))

(event EventStopFire
  (params (Character :type STU%20Base%20Character%20Object%20Reference)))

(fn ConstructionScript)

(fn Fire
  (if (Class|STUBaseWeapon|IsAmmoEmpty)
    (Audio|SpawnSoundatLocation (Variables|Default|GetNoAmmoSound) (Transformation|GetActorLocation) "0, 0, 0" 1.0 1.0 0.0 0 0)
    (else
      (Class|STUBaseWeapon|SpawnMuzzleFX)
      (Class|STUBaseWeapon|DecreaseAmmo)
      (if (Networking|IsServer)
        (bind _direction (CallFunction|GetProjectileDirection))
        (bind _returnvalue (Game|SpawnActorfromClass (Variables|Default|GetProjectileClass) (Math|Transform|MakeTransform (Class|STUBaseWeapon|GetMuzzleWorldLocation) "0, 0, 0" "1.000000,1.000000,1.000000") "AlwaysSpawn" "MultiplyWithRoot" (Components|GetOwner) _direction 0))
        (Default|InitVelocityMulticast _returnvalue (* _direction (Variables|Default|GetProjectile%20%20Speed)))))))

(fn GetProjectileDirection
  (bind (_tracestart _traceend) (Class|STUBaseWeapon|GetTraceData))
  (bind _hitresult (Class|STUBaseWeapon|MakeHit _tracestart _traceend))
  (return (Math|Vector|Normalize (- (Math|Vector|SelectVector (.ImpactPoint (Collision|BreakHitResult _hitresult)) _traceend (.bBlockingHit (Collision|BreakHitResult _hitresult))) (Class|STUBaseWeapon|GetMuzzleWorldLocation)))))