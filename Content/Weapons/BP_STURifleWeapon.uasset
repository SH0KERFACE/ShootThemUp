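; Networked automatic rifle weapon that fires hitscan shots on a looping timer until stopped or out of ammo.
; Each shot traces from the player's view, draws a Niagara tracer from the muzzle and decreases ammo on server and owning client.
; The server alone applies damage and multicasts the tracer to other clients.
; Muzzle effect and fire sound references are cached and toggled as firing starts and stops.
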(event Custom|SpawnTraceFX_Multicast
  (params (TraceStart :type Vector) (TraceEnd :type Vector) (Char :type Pawn%20Object%20Reference))
  (if (not (or (Networking|IsServer) (Pawn|IsLocallyControlled Char)))
    (CallFunction|SpawnTraceFX TraceStart TraceEnd)))

(event EventStartFire
  (params (Character :type STU%20Base%20Character%20Object%20Reference))
  (Variables|Default|SetCharacter Character)
  (CallFunction|InitFX)
  (if (not (Utilities|Time|IsTimerActivebyHandle (Variables|Default|GetFireTimer)))
    (CallFunction|Fire)
    (bind _returnvalue (Utilities|Time|SetTimerbyFunctionName 0 "Fire" (Variables|Default|GetTimeBetwenShots) true))
    (Variables|Default|SetFireTimer _returnvalue)))

(event EventStopFire
  (params (Character :type STU%20Base%20Character%20Object%20Reference))
  (CallFunction|SetFXActive false)
  (Utilities|Time|ClearandInvalidateTimerbyHandle (Variables|Default|GetFireTimer)))

(fn ConstructionScript)

(fn InitFX
  (Utilities|IsValid (Variables|Default|GetMuzzleEffect)
    (:Is%20Valid
      _)
    (:Is%20Not%20Valid
      (bind _returnvalue (Class|STUBaseWeapon|SpawnMuzzleFX))
      (Variables|Default|SetMuzzleEffect _returnvalue)))
  (bind _returnvalue_2 (Audio|SpawnSoundAttached (Variables|Default|GetFireSound) (Variables|Default|GetWeaponMesh) (Variables|Default|GetMuzzleSocketName) "0, 0, 0" "0, 0, 0" "KeepRelativeOffset" false 1.0 1.0 0.0 0 0))
  (Utilities|IsValid (Variables|Default|GetFireSoundEffect)
    (:Is%20Valid
      _)
    (:Is%20Not%20Valid
      (Variables|Default|SetFireSoundEffect _returnvalue_2)))
  (CallFunction|SetFXActive true))

(fn SetFXActive
  (params (IsActive :type Boolean))
  (bind _muzzleeffect (Variables|Default|GetMuzzleEffect))
  (bind _firesoundeffect (Variables|Default|GetFireSoundEffect))
  (Utilities|IsValid _muzzleeffect
    (:Is%20Valid
      (Class|NiagaraComponent|SetPaused _muzzleeffect (not IsActive))
      (Rendering|SetVisibility _muzzleeffect IsActive false))
    (:Is%20Not%20Valid
      _))
  (Utilities|IsValid _firesoundeffect
    (:Is%20Valid
      (if IsActive
        (Audio|Components|Audio|Play (Variables|Default|GetFireSoundEffect) 0.0)
        (else
          (Audio|Components|Audio|Stop _firesoundeffect))))))

(fn Fire
  (bind _returnvalue (Class|STUBaseWeapon|GetMuzzleWorldLocation))
  (bind _character (Variables|Default|GetCharacter))
  (bind _character_2 (Variables|Default|GetCharacter))
  (bind _weaponcomponent (Variables|/Script/ShootThemUp.STUBaseCharacter|GetWeaponComponent _character))
  (bind _currentweapon (Variables|/Script/ShootThemUp.STUWeaponComponent|GetCurrentWeapon _weaponcomponent))
  (bind (_viewlocation _returnvalue_2) (CallFunction|GetTraceLocations _currentweapon))
  (if (Class|STUBaseWeapon|IsAmmoEmpty _currentweapon)
    (Class|STUBaseWeapon|StopFire _currentweapon _character)
    (elif (or (Pawn|IsLocallyControlled _character) (Networking|IsServer))
      (bind _hitresult (Class|STUBaseWeapon|MakeHit _currentweapon _viewlocation _returnvalue_2))
      (CallFunction|SpawnTraceFX _returnvalue (.ImpactPoint (Collision|BreakHitResult _hitresult)))
      (Class|STUBaseWeapon|DecreaseAmmo)
      (if (Networking|IsServer)
        (CallFunction|SpawnTraceFXMulticast _returnvalue (.ImpactPoint (Collision|BreakHitResult _hitresult)) _character_2)
        (Utilities|IsValid (.HitActor (Collision|BreakHitResult _hitresult))
          (:Is%20Valid
            (Game|Damage|ApplyDamage (.HitActor (Collision|BreakHitResult _hitresult)) (Variables|Default|GetDamage) (Pawn|GetController _character_2) self)))))))

(fn SpawnTraceFX
  (params (TraceStart :type Vector) (TraceEnd :type Vector))
  (bind _returnvalue (Niagara|SpawnSystematLocation (Variables|Default|GetTraceFX) TraceStart))
  (Utilities|IsValid _returnvalue
    (:Is%20Valid
      (Niagara|SetNiagaraVariable(Vector3) _returnvalue (Variables|Default|GetTraceTargetName) TraceEnd))))

(fn GetTraceLocations
  (params (Weapon :type STU%20Base%20Weapon%20Object%20Reference))
  (bind (_viewlocation _viewrotation) (Class|STUBaseWeapon|GetPlayerViewPoint Weapon))
  (return _viewlocation (+ (.TraceStart (Class|STUBaseWeapon|GetTraceData Weapon)) (* (Math|Vector|GetForwardVector _viewrotation) (Variables|Default|GetTraceMaxDistance)))))